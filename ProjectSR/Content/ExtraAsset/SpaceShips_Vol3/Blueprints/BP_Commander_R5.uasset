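; Commander R5 spaceship Blueprint with a selectable hull color and adjustable thruster glow.
; The construction script picks the hull material, and for some colors a thruster tint, then creates dynamic material instances for the hull and four shared flare layers.
; A Thrust value drives hull glow, flare opacity and thruster mesh stretch.
; With AnimateThrustersDemo enabled, BeginPlay waits a color-based delay, then animates Thrust through a timeline.
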(event `self.ReceiveBeginPlay`
  (if (`self.AnimateThrusters_Demo`)
    (`KismetSystemLibrary.Delay` (* (`self.Color`) 0.4))
    (bind (_direction _thrust) (`Timeline|Timeline_0`)
      (:`Update`
        (set `self.Thrust` _thrust)
        (`self.Adjust Thrusters`)))))

(fn `Adjust Thrusters`
  (bind _thrust (`self.Thrust`))
  ;[1 1 1] Adjust Thruster Intensity
  (`MaterialInstanceDynamic.SetScalarParameterValue` (`self.ShipMaterial`) "Thrust" (`KismetMathLibrary.Lerp` 0.0 3.0 _thrust))
  (`SceneComponent.SetRelativeScale3D` (`self.SM_RocketFlare_TL`) (`KismetMathLibrary.MakeVector` 1.0 (`KismetMathLibrary.Lerp` 0.0 1.7 _thrust) 1.0))
  (`SceneComponent.SetRelativeScale3D` (`self.SM_RocketFlare_BL`) (`KismetMathLibrary.MakeVector` 1.0 (`KismetMathLibrary.Lerp` 0.0 1.7 _thrust) 1.0))
  (`SceneComponent.SetRelativeScale3D` (`self.SM_RocketFlare_TR`) (`KismetMathLibrary.MakeVector` 1.0 (`KismetMathLibrary.Lerp` 0.0 1.7 _thrust) 1.0))
  (`SceneComponent.SetRelativeScale3D` (`self.SM_RocketFlare_BR`) (`KismetMathLibrary.MakeVector` 1.0 (`KismetMathLibrary.Lerp` 0.0 1.7 _thrust) 1.0))
  (`SceneComponent.SetRelativeScale3D` (`self.SM_Commander_R5_Thruster_B_L`) (`KismetMathLibrary.MakeVector` 1.0 (`KismetMathLibrary.Lerp` 0.0 1.7 _thrust) 1.0))
  (`SceneComponent.SetRelativeScale3D` (`self.SM_Commander_R5_Thruster_B_R`) (`KismetMathLibrary.MakeVector` -1.0 (`KismetMathLibrary.Lerp` 0.0 1.7 _thrust) 1.0))
  (`MaterialInstanceDynamic.SetScalarParameterValue` (`self.DynMat_RocketFlare0`) "Opacity" (`self.Thrust`))
  (`MaterialInstanceDynamic.SetScalarParameterValue` (`self.DynMat_RocketFlare1`) "Opacity" (`self.Thrust`))
  (`MaterialInstanceDynamic.SetScalarParameterValue` (`self.DynMat_RocketFlare2`) "Opacity" (`self.Thrust`))
  (`MaterialInstanceDynamic.SetScalarParameterValue` (`self.DynMat_RocketFlare3`) "Opacity" (`self.Thrust`)))

(fn `UserConstructionScript`
  (bind _sm_commander_r5 (`self.SM_Commander_R5`))
  (bind _sm_commander_r5_thruster_b_l (`self.SM_Commander_R5_Thruster_B_L`))
  (bind _sm_commander_r5_2 (`self.SM_Commander_R5`))
  (bind _returnvalue (`KismetMaterialLibrary.CreateDynamicMaterialInstance` "/Game/ExtraAsset/SpaceShips_Vol3/Materials/RocketFlare/MI_RocketFlare_0.MI_RocketFlare_0"))
  (set `self.DynMat_RocketFlare0` _returnvalue)
  (bind _returnvalue_2 (`KismetMaterialLibrary.CreateDynamicMaterialInstance` "/Game/ExtraAsset/SpaceShips_Vol3/Materials/RocketFlare/MI_RocketFlare_1.MI_RocketFlare_1"))
  (set `self.DynMat_RocketFlare1` _returnvalue_2)
  (bind _returnvalue_3 (`KismetMaterialLibrary.CreateDynamicMaterialInstance` "/Game/ExtraAsset/SpaceShips_Vol3/Materials/RocketFlare/MI_RocketFlare_2.MI_RocketFlare_2"))
  (set `self.DynMat_RocketFlare2` _returnvalue_3)
  (bind _returnvalue_4 (`KismetMaterialLibrary.CreateDynamicMaterialInstance` "/Game/ExtraAsset/SpaceShips_Vol3/Materials/RocketFlare/MI_RocketFlare_3.MI_RocketFlare_3"))
  (set `self.DynMat_RocketFlare3` _returnvalue_4)
  (`PrimitiveComponent.SetMaterial` _sm_commander_r5_thruster_b_l 0 (`self.DynMat_RocketFlare0`))
  (`PrimitiveComponent.SetMaterial` (`self.SM_Commander_R5_Thruster_B_R`) 0 (`self.DynMat_RocketFlare0`))
  (`PrimitiveComponent.SetMaterial` (`self.SM_RocketFlare_TL`) 0 (`self.DynMat_RocketFlare0`))
  (`PrimitiveComponent.SetMaterial` (`self.SM_RocketFlare_BL`) 0 (`self.DynMat_RocketFlare0`))
  (`PrimitiveComponent.SetMaterial` (`self.SM_RocketFlare_TR`) 0 (`self.DynMat_RocketFlare0`))
  (`PrimitiveComponent.SetMaterial` (`self.SM_RocketFlare_BR`) 0 (`self.DynMat_RocketFlare0`))
  (`PrimitiveComponent.SetMaterial` _sm_commander_r5_thruster_b_l 1 (`self.DynMat_RocketFlare1`))
  (`PrimitiveComponent.SetMaterial` (`self.SM_Commander_R5_Thruster_B_R`) 1 (`self.DynMat_RocketFlare1`))
  (`PrimitiveComponent.SetMaterial` (`self.SM_RocketFlare_TL`) 1 (`self.DynMat_RocketFlare1`))
  (`PrimitiveComponent.SetMaterial` (`self.SM_RocketFlare_BL`) 1 (`self.DynMat_RocketFlare1`))
  (`PrimitiveComponent.SetMaterial` (`self.SM_RocketFlare_TR`) 1 (`self.DynMat_RocketFlare1`))
  (`PrimitiveComponent.SetMaterial` (`self.SM_RocketFlare_BR`) 1 (`self.DynMat_RocketFlare1`))
  (`PrimitiveComponent.SetMaterial` _sm_commander_r5_thruster_b_l 2 (`self.DynMat_RocketFlare2`))
  (`PrimitiveComponent.SetMaterial` (`self.SM_Commander_R5_Thruster_B_R`) 2 (`self.DynMat_RocketFlare2`))
  (`PrimitiveComponent.SetMaterial` (`self.SM_RocketFlare_TL`) 2 (`self.DynMat_RocketFlare2`))
  (`PrimitiveComponent.SetMaterial` (`self.SM_RocketFlare_BL`) 2 (`self.DynMat_RocketFlare2`))
  (`PrimitiveComponent.SetMaterial` (`self.SM_RocketFlare_TR`) 2 (`self.DynMat_RocketFlare2`))
  (`PrimitiveComponent.SetMaterial` (`self.SM_RocketFlare_BR`) 2 (`self.DynMat_RocketFlare2`))
  (`PrimitiveComponent.SetMaterial` _sm_commander_r5_thruster_b_l 3 (`self.DynMat_RocketFlare3`))
  (`PrimitiveComponent.SetMaterial` (`self.SM_Commander_R5_Thruster_B_R`) 3 (`self.DynMat_RocketFlare3`))
  (`PrimitiveComponent.SetMaterial` (`self.SM_RocketFlare_TL`) 3 (`self.DynMat_RocketFlare3`))
  (`PrimitiveComponent.SetMaterial` (`self.SM_RocketFlare_BL`) 3 (`self.DynMat_RocketFlare3`))
  (`PrimitiveComponent.SetMaterial` (`self.SM_RocketFlare_TR`) 3 (`self.DynMat_RocketFlare3`))
  (`PrimitiveComponent.SetMaterial` (`self.SM_RocketFlare_BR`) 3 (`self.DynMat_RocketFlare3`))
  (switch `int` (`self.Color`)
    (:`0`
      (`PrimitiveComponent.SetMaterial` _sm_commander_r5_2 0 "/Game/ExtraAsset/SpaceShips_Vol3/Materials/Commander_R5/MI_Commander_R5_Black.MI_Commander_R5_Black")
      (set `self.Thruster_Color` (struct :`R` 1.0 :`B` 0.027019 :`A` 1.0)))
    (:`1`
      (`PrimitiveComponent.SetMaterial` _sm_commander_r5_2 0 "/Game/ExtraAsset/SpaceShips_Vol3/Materials/Commander_R5/MI_Commander_R5_White.MI_Commander_R5_White")
      (set `self.Thruster_Color` (struct :`G` 0.269754 :`B` 1.0 :`A` 1.0)))
    (:`2`
      (`PrimitiveComponent.SetMaterial` _sm_commander_r5_2 0 "/Game/ExtraAsset/SpaceShips_Vol3/Materials/Commander_R5/MI_Commander_R5_Yellow.MI_Commander_R5_Yellow")
      (set `self.Thruster_Color` (struct :`R` 0.59 :`G` 0.957398 :`B` 1.0 :`A` 1.0)))
    (:`3`
      (`PrimitiveComponent.SetMaterial` _sm_commander_r5_2 0 "/Game/ExtraAsset/SpaceShips_Vol3/Materials/Commander_R5/MI_Commander_R5_Green.MI_Commander_R5_Green"))
    (:`4`
      (`PrimitiveComponent.SetMaterial` _sm_commander_r5_2 0 "/Game/ExtraAsset/SpaceShips_Vol3/Materials/Commander_R5/MI_Commander_R5_Red.MI_Commander_R5_Red"))
    (:`5`
      (`PrimitiveComponent.SetMaterial` _sm_commander_r5_2 0 "/Game/ExtraAsset/SpaceShips_Vol3/Materials/Commander_R5/MI_Commander_R5_Blue.MI_Commander_R5_Blue")
      (set `self.Thruster_Color` (struct :`G` 0.488851 :`B` 1.0 :`A` 1.0))))
  (bind _returnvalue_5 (`PrimitiveComponent.CreateDynamicMaterialInstance` _sm_commander_r5 0 (`PrimitiveComponent.GetMaterial` _sm_commander_r5 0) "None"))
  (bind _output_get (set `self.ShipMaterial` _returnvalue_5))
  (`PrimitiveComponent.SetMaterial` _sm_commander_r5 0 _output_get)
  (`self.Adjust Thrusters`)
  (`MaterialInstanceDynamic.SetVectorParameterValue` (`self.DynMat_RocketFlare0`) "Color" (`self.Thruster_Color`))
  (`MaterialInstanceDynamic.SetVectorParameterValue` (`self.DynMat_RocketFlare1`) "Color" (`self.Thruster_Color`))
  (`MaterialInstanceDynamic.SetVectorParameterValue` (`self.DynMat_RocketFlare2`) "Color" (`self.Thruster_Color`))
  (`MaterialInstanceDynamic.SetVectorParameterValue` (`self.DynMat_RocketFlare3`) "Color" (`self.Thruster_Color`))
  (`MaterialInstanceDynamic.SetVectorParameterValue` (`self.ShipMaterial`) "ThrusterColor" (`self.Thruster_Color`)))