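; Destroyer RF3 spaceship actor with a selectable hull color and adjustable thruster effects.
; The construction script picks the hull material and, for some colors, a thruster color, then creates dynamic materials for the hull and shared rocket flares.
; Thrust scales the thruster meshes and drives flare opacity and hull glow.
; With AnimateThrustersDemo on, BeginPlay waits a color-based delay, then a timeline animates Thrust.
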(event `self.ReceiveBeginPlay`
  (if (`self.AnimateThrusters_Demo`)
    (`KismetSystemLibrary.Delay` (* (`self.Color`) 0.4))
    (bind (_direction _thrust) (`Timeline|Timeline_0`)
      (:`Update`
        (set `self.Thrust` _thrust)
        (`self.Adjust Thrusters`)))))

(fn `Adjust Thrusters`
  (bind _thrust (`self.Thrust`))
  ;[1 1 1] Adjust Thruster Intensity
  (`MaterialInstanceDynamic.SetScalarParameterValue` (`self.ShipMaterial`) "Thrust" (`KismetMathLibrary.Lerp` 0.0 10.0 _thrust))
  (`SceneComponent.SetRelativeScale3D` (`self.SM_Frigate_MB3_Thruster_TL2`) (`KismetMathLibrary.MakeVector` (`KismetMathLibrary.Lerp` 0.0 60.0 _thrust) 19.0 19.0))
  (`SceneComponent.SetRelativeScale3D` (`self.SM_Frigate_MB3_Thruster_BL2`) (`KismetMathLibrary.MakeVector` (`KismetMathLibrary.Lerp` 0.0 60.0 _thrust) 19.0 19.0))
  (`SceneComponent.SetRelativeScale3D` (`self.SM_Frigate_MB3_Thruster_BL1`) (`KismetMathLibrary.MakeVector` (`KismetMathLibrary.Lerp` 0.0 60.0 _thrust) 19.0 19.0))
  (`SceneComponent.SetRelativeScale3D` (`self.SM_Frigate_MB3_Thruster_TL1`) (`KismetMathLibrary.MakeVector` (`KismetMathLibrary.Lerp` 0.0 60.0 _thrust) 19.0 19.0))
  (`SceneComponent.SetRelativeScale3D` (`self.SM_Frigate_MB3_Thruster_TR1`) (`KismetMathLibrary.MakeVector` (`KismetMathLibrary.Lerp` 0.0 60.0 _thrust) 19.0 19.0))
  (`SceneComponent.SetRelativeScale3D` (`self.SM_Frigate_MB3_Thruster_TR2`) (`KismetMathLibrary.MakeVector` (`KismetMathLibrary.Lerp` 0.0 60.0 _thrust) 19.0 19.0))
  (`SceneComponent.SetRelativeScale3D` (`self.SM_Frigate_MB3_Thruster_BR2`) (`KismetMathLibrary.MakeVector` (`KismetMathLibrary.Lerp` 0.0 60.0 _thrust) 19.0 19.0))
  (`SceneComponent.SetRelativeScale3D` (`self.SM_Frigate_MB3_Thruster_BR1`) (`KismetMathLibrary.MakeVector` (`KismetMathLibrary.Lerp` 0.0 60.0 _thrust) 19.0 19.0))
  (`SceneComponent.SetRelativeScale3D` (`self.SM_Frigate_MB3_Thruster_M_L`) (`KismetMathLibrary.MakeVector` (`KismetMathLibrary.Lerp` 0.0 40.0 _thrust) 13.0 13.0))
  (`SceneComponent.SetRelativeScale3D` (`self.SM_Frigate_MB3_Thruster_M_R`) (`KismetMathLibrary.MakeVector` (`KismetMathLibrary.Lerp` 0.0 40.0 _thrust) 13.0 13.0))
  (`MaterialInstanceDynamic.SetScalarParameterValue` (`self.DynMat_RocketFlare0`) "Opacity" (`self.Thrust`))
  (`MaterialInstanceDynamic.SetScalarParameterValue` (`self.DynMat_RocketFlare1`) "Opacity" (`self.Thrust`))
  (`MaterialInstanceDynamic.SetScalarParameterValue` (`self.DynMat_RocketFlare2`) "Opacity" (`self.Thrust`))
  (`MaterialInstanceDynamic.SetScalarParameterValue` (`self.DynMat_RocketFlare3`) "Opacity" (`self.Thrust`)))

(fn `UserConstructionScript`
  (bind _sm_frigate_mb3_thruster_tl2 (`self.SM_Frigate_MB3_Thruster_TL2`))
  (bind _sm_destroyer_rf3 (`self.SM_Destroyer_RF3`))
  (bind _sm_destroyer_rf3_2 (`self.SM_Destroyer_RF3`))
  (bind _returnvalue (`KismetMaterialLibrary.CreateDynamicMaterialInstance` "/Game/ExtraAsset/SpaceShips_Vol3/Materials/RocketFlare/MI_RocketFlare_0.MI_RocketFlare_0"))
  (set `self.DynMat_RocketFlare0` _returnvalue)
  (bind _returnvalue_2 (`KismetMaterialLibrary.CreateDynamicMaterialInstance` "/Game/ExtraAsset/SpaceShips_Vol3/Materials/RocketFlare/MI_RocketFlare_1.MI_RocketFlare_1"))
  (set `self.DynMat_RocketFlare1` _returnvalue_2)
  (bind _returnvalue_3 (`KismetMaterialLibrary.CreateDynamicMaterialInstance` "/Game/ExtraAsset/SpaceShips_Vol3/Materials/RocketFlare/MI_RocketFlare_2.MI_RocketFlare_2"))
  (set `self.DynMat_RocketFlare2` _returnvalue_3)
  (bind _returnvalue_4 (`KismetMaterialLibrary.CreateDynamicMaterialInstance` "/Game/ExtraAsset/SpaceShips_Vol3/Materials/RocketFlare/MI_RocketFlare_3.MI_RocketFlare_3"))
  (set `self.DynMat_RocketFlare3` _returnvalue_4)
  (`PrimitiveComponent.SetMaterial` _sm_frigate_mb3_thruster_tl2 0 (`self.DynMat_RocketFlare0`))
  (`PrimitiveComponent.SetMaterial` (`self.SM_Frigate_MB3_Thruster_BL2`) 0 (`self.DynMat_RocketFlare0`))
  (`PrimitiveComponent.SetMaterial` (`self.SM_Frigate_MB3_Thruster_BL1`) 0 (`self.DynMat_RocketFlare0`))
  (`PrimitiveComponent.SetMaterial` (`self.SM_Frigate_MB3_Thruster_TL1`) 0 (`self.DynMat_RocketFlare0`))
  (`PrimitiveComponent.SetMaterial` (`self.SM_Frigate_MB3_Thruster_M_L`) 0 (`self.DynMat_RocketFlare0`))
  (`PrimitiveComponent.SetMaterial` (`self.SM_Frigate_MB3_Thruster_TR1`) 0 (`self.DynMat_RocketFlare0`))
  (`PrimitiveComponent.SetMaterial` (`self.SM_Frigate_MB3_Thruster_TR2`) 0 (`self.DynMat_RocketFlare0`))
  (`PrimitiveComponent.SetMaterial` (`self.SM_Frigate_MB3_Thruster_BR2`) 0 (`self.DynMat_RocketFlare0`))
  (`PrimitiveComponent.SetMaterial` (`self.SM_Frigate_MB3_Thruster_BR1`) 0 (`self.DynMat_RocketFlare0`))
  (`PrimitiveComponent.SetMaterial` (`self.SM_Frigate_MB3_Thruster_M_R`) 0 (`self.DynMat_RocketFlare0`))
  (`PrimitiveComponent.SetMaterial` _sm_frigate_mb3_thruster_tl2 1 (`self.DynMat_RocketFlare1`))
  (`PrimitiveComponent.SetMaterial` (`self.SM_Frigate_MB3_Thruster_BL2`) 1 (`self.DynMat_RocketFlare1`))
  (`PrimitiveComponent.SetMaterial` (`self.SM_Frigate_MB3_Thruster_BL1`) 1 (`self.DynMat_RocketFlare1`))
  (`PrimitiveComponent.SetMaterial` (`self.SM_Frigate_MB3_Thruster_TL1`) 1 (`self.DynMat_RocketFlare1`))
  (`PrimitiveComponent.SetMaterial` (`self.SM_Frigate_MB3_Thruster_M_L`) 1 (`self.DynMat_RocketFlare1`))
  (`PrimitiveComponent.SetMaterial` (`self.SM_Frigate_MB3_Thruster_TR1`) 1 (`self.DynMat_RocketFlare1`))
  (`PrimitiveComponent.SetMaterial` (`self.SM_Frigate_MB3_Thruster_TR2`) 1 (`self.DynMat_RocketFlare1`))
  (`PrimitiveComponent.SetMaterial` (`self.SM_Frigate_MB3_Thruster_BR2`) 1 (`self.DynMat_RocketFlare1`))
  (`PrimitiveComponent.SetMaterial` (`self.SM_Frigate_MB3_Thruster_BR1`) 1 (`self.DynMat_RocketFlare1`))
  (`PrimitiveComponent.SetMaterial` (`self.SM_Frigate_MB3_Thruster_M_R`) 1 (`self.DynMat_RocketFlare1`))
  (`PrimitiveComponent.SetMaterial` _sm_frigate_mb3_thruster_tl2 2 (`self.DynMat_RocketFlare2`))
  (`PrimitiveComponent.SetMaterial` (`self.SM_Frigate_MB3_Thruster_BL2`) 2 (`self.DynMat_RocketFlare2`))
  (`PrimitiveComponent.SetMaterial` (`self.SM_Frigate_MB3_Thruster_BL1`) 2 (`self.DynMat_RocketFlare2`))
  (`PrimitiveComponent.SetMaterial` (`self.SM_Frigate_MB3_Thruster_TL1`) 2 (`self.DynMat_RocketFlare2`))
  (`PrimitiveComponent.SetMaterial` (`self.SM_Frigate_MB3_Thruster_M_L`) 2 (`self.DynMat_RocketFlare2`))
  (`PrimitiveComponent.SetMaterial` (`self.SM_Frigate_MB3_Thruster_TR1`) 2 (`self.DynMat_RocketFlare2`))
  (`PrimitiveComponent.SetMaterial` (`self.SM_Frigate_MB3_Thruster_TR2`) 2 (`self.DynMat_RocketFlare2`))
  (`PrimitiveComponent.SetMaterial` (`self.SM_Frigate_MB3_Thruster_BR2`) 2 (`self.DynMat_RocketFlare2`))
  (`PrimitiveComponent.SetMaterial` (`self.SM_Frigate_MB3_Thruster_BR1`) 2 (`self.DynMat_RocketFlare2`))
  (`PrimitiveComponent.SetMaterial` (`self.SM_Frigate_MB3_Thruster_M_R`) 2 (`self.DynMat_RocketFlare2`))
  (`PrimitiveComponent.SetMaterial` _sm_frigate_mb3_thruster_tl2 3 (`self.DynMat_RocketFlare3`))
  (`PrimitiveComponent.SetMaterial` (`self.SM_Frigate_MB3_Thruster_BL2`) 3 (`self.DynMat_RocketFlare3`))
  (`PrimitiveComponent.SetMaterial` (`self.SM_Frigate_MB3_Thruster_BL1`) 3 (`self.DynMat_RocketFlare3`))
  (`PrimitiveComponent.SetMaterial` (`self.SM_Frigate_MB3_Thruster_TL1`) 3 (`self.DynMat_RocketFlare3`))
  (`PrimitiveComponent.SetMaterial` (`self.SM_Frigate_MB3_Thruster_M_L`) 3 (`self.DynMat_RocketFlare3`))
  (`PrimitiveComponent.SetMaterial` (`self.SM_Frigate_MB3_Thruster_TR1`) 3 (`self.DynMat_RocketFlare3`))
  (`PrimitiveComponent.SetMaterial` (`self.SM_Frigate_MB3_Thruster_TR2`) 3 (`self.DynMat_RocketFlare3`))
  (`PrimitiveComponent.SetMaterial` (`self.SM_Frigate_MB3_Thruster_BR2`) 3 (`self.DynMat_RocketFlare3`))
  (`PrimitiveComponent.SetMaterial` (`self.SM_Frigate_MB3_Thruster_BR1`) 3 (`self.DynMat_RocketFlare3`))
  (`PrimitiveComponent.SetMaterial` (`self.SM_Frigate_MB3_Thruster_M_R`) 3 (`self.DynMat_RocketFlare3`))
  (switch `int` (`self.Color`)
    (:`0`
      (`PrimitiveComponent.SetMaterial` _sm_destroyer_rf3_2 0 "/Game/ExtraAsset/SpaceShips_Vol3/Materials/Destroyer_RF3/MI_Destroyer_RF3_Black.MI_Destroyer_RF3_Black")
      (set `self.Thruster_Color` (struct :`R` 1.0 :`B` 0.027019 :`A` 1.0)))
    (:`1`
      (`PrimitiveComponent.SetMaterial` _sm_destroyer_rf3_2 0 "/Game/ExtraAsset/SpaceShips_Vol3/Materials/Destroyer_RF3/MI_Destroyer_RF3_White.MI_Destroyer_RF3_White"))
    (:`2`
      (`PrimitiveComponent.SetMaterial` _sm_destroyer_rf3_2 0 "/Game/ExtraAsset/SpaceShips_Vol3/Materials/Destroyer_RF3/MI_Destroyer_RF3_Yellow.MI_Destroyer_RF3_Yellow")
      (set `self.Thruster_Color` (struct :`R` 1.0 :`G` 0.978421 :`B` 0.72 :`A` 1.0)))
    (:`3`
      (`PrimitiveComponent.SetMaterial` _sm_destroyer_rf3_2 0 "/Game/ExtraAsset/SpaceShips_Vol3/Materials/Destroyer_RF3/MI_Destroyer_RF3_Green.MI_Destroyer_RF3_Green")
      (set `self.Thruster_Color` (struct :`G` 1.0 :`B` 0.89897 :`A` 1.0)))
    (:`4`
      (`PrimitiveComponent.SetMaterial` _sm_destroyer_rf3_2 0 "/Game/ExtraAsset/SpaceShips_Vol3/Materials/Destroyer_RF3/MI_Destroyer_RF3_Red.MI_Destroyer_RF3_Red"))
    (:`5`
      (`PrimitiveComponent.SetMaterial` _sm_destroyer_rf3_2 0 "/Game/ExtraAsset/SpaceShips_Vol3/Materials/Destroyer_RF3/MI_Destroyer_RF3_Blue.MI_Destroyer_RF3_Blue")))
  (bind _returnvalue_5 (`PrimitiveComponent.CreateDynamicMaterialInstance` _sm_destroyer_rf3 0 (`PrimitiveComponent.GetMaterial` _sm_destroyer_rf3 0) "None"))
  (bind _output_get (set `self.ShipMaterial` _returnvalue_5))
  (`PrimitiveComponent.SetMaterial` _sm_destroyer_rf3 0 _output_get)
  (`self.Adjust Thrusters`)
  (`MaterialInstanceDynamic.SetVectorParameterValue` (`self.DynMat_RocketFlare0`) "Color" (`self.Thruster_Color`))
  (`MaterialInstanceDynamic.SetVectorParameterValue` (`self.DynMat_RocketFlare1`) "Color" (`self.Thruster_Color`))
  (`MaterialInstanceDynamic.SetVectorParameterValue` (`self.DynMat_RocketFlare2`) "Color" (`self.Thruster_Color`))
  (`MaterialInstanceDynamic.SetVectorParameterValue` (`self.DynMat_RocketFlare3`) "Color" (`self.Thruster_Color`))
  (`MaterialInstanceDynamic.SetVectorParameterValue` (`self.ShipMaterial`) "ThrusterColor" (`self.Thruster_Color`)))