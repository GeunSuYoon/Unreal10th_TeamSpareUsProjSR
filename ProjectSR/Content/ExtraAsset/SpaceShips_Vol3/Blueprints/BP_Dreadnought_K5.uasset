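; Dreadnought K5 spaceship display actor with selectable hull color variants and animated engine thrusters.
; The construction script creates dynamic flare and hull materials, picks the hull skin from Color and applies a thruster tint, overridden for some variants.
; When AnimateThrustersDemo is set, BeginPlay waits a Color-scaled delay, then a timeline drives Thrust.
; AdjustThrusters maps Thrust to hull glow, thruster mesh length and flare opacity.
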(event `self.ReceiveBeginPlay`
  (if (`self.AnimateThrusters_Demo`)
    (`KismetSystemLibrary.Delay` (* (`self.Color`) 0.4))
    (bind (_direction _thrust) (`Timeline|Timeline_0`)
      (:`Update`
        (set `self.Thrust` _thrust)
        (`self.Adjust Thrusters`)))))

(fn `Adjust Thrusters`
  (bind _thrust (`self.Thrust`))
  (bind _returnvalue (`KismetMathLibrary.Lerp` 0.0 100.0 _thrust))
  ;[1 1 1] Adjust Thruster Intensity
  (`MaterialInstanceDynamic.SetScalarParameterValue` (`self.ShipMaterial`) "Thrust" (`KismetMathLibrary.Lerp` 0.0 6.0 _thrust))
  (`SceneComponent.SetRelativeScale3D` (`self.SM_Frigate_MB3_Thruster_L1`) (`KismetMathLibrary.MakeVector` _returnvalue 32.0 32.0))
  (`SceneComponent.SetRelativeScale3D` (`self.SM_Frigate_MB3_Thruster_R1`) (`KismetMathLibrary.MakeVector` _returnvalue 32.0 32.0))
  (`SceneComponent.SetRelativeScale3D` (`self.SM_Frigate_MB3_Thruster_R2`) (`KismetMathLibrary.MakeVector` _returnvalue 27.0 27.0))
  (`SceneComponent.SetRelativeScale3D` (`self.SM_Frigate_MB3_Thruster_L2`) (`KismetMathLibrary.MakeVector` _returnvalue 27.0 27.0))
  (`MaterialInstanceDynamic.SetScalarParameterValue` (`self.DynMat_RocketFlare0`) "Opacity" (`self.Thrust`))
  (`MaterialInstanceDynamic.SetScalarParameterValue` (`self.DynMat_RocketFlare1`) "Opacity" (`self.Thrust`))
  (`MaterialInstanceDynamic.SetScalarParameterValue` (`self.DynMat_RocketFlare2`) "Opacity" (`self.Thrust`))
  (`MaterialInstanceDynamic.SetScalarParameterValue` (`self.DynMat_RocketFlare3`) "Opacity" (`self.Thrust`)))

(fn `UserConstructionScript`
  (bind _sm_dreadnought_k5 (`self.SM_Dreadnought_K5`))
  (bind _sm_frigate_mb3_thruster_l2 (`self.SM_Frigate_MB3_Thruster_L2`))
  (bind _sm_dreadnought_k5_2 (`self.SM_Dreadnought_K5`))
  (bind _returnvalue (`KismetMaterialLibrary.CreateDynamicMaterialInstance` "/Game/ExtraAsset/SpaceShips_Vol3/Materials/RocketFlare/MI_RocketFlare_0.MI_RocketFlare_0"))
  (set `self.DynMat_RocketFlare0` _returnvalue)
  (bind _returnvalue_2 (`KismetMaterialLibrary.CreateDynamicMaterialInstance` "/Game/ExtraAsset/SpaceShips_Vol3/Materials/RocketFlare/MI_RocketFlare_1.MI_RocketFlare_1"))
  (set `self.DynMat_RocketFlare1` _returnvalue_2)
  (bind _returnvalue_3 (`KismetMaterialLibrary.CreateDynamicMaterialInstance` "/Game/ExtraAsset/SpaceShips_Vol3/Materials/RocketFlare/MI_RocketFlare_2.MI_RocketFlare_2"))
  (set `self.DynMat_RocketFlare2` _returnvalue_3)
  (bind _returnvalue_4 (`KismetMaterialLibrary.CreateDynamicMaterialInstance` "/Game/ExtraAsset/SpaceShips_Vol3/Materials/RocketFlare/MI_RocketFlare_3.MI_RocketFlare_3"))
  (set `self.DynMat_RocketFlare3` _returnvalue_4)
  (`PrimitiveComponent.SetMaterial` _sm_frigate_mb3_thruster_l2 0 (`self.DynMat_RocketFlare0`))
  (`PrimitiveComponent.SetMaterial` (`self.SM_Frigate_MB3_Thruster_L1`) 0 (`self.DynMat_RocketFlare0`))
  (`PrimitiveComponent.SetMaterial` (`self.SM_Frigate_MB3_Thruster_R1`) 0 (`self.DynMat_RocketFlare0`))
  (`PrimitiveComponent.SetMaterial` (`self.SM_Frigate_MB3_Thruster_R2`) 0 (`self.DynMat_RocketFlare0`))
  (`PrimitiveComponent.SetMaterial` _sm_frigate_mb3_thruster_l2 1 (`self.DynMat_RocketFlare1`))
  (`PrimitiveComponent.SetMaterial` (`self.SM_Frigate_MB3_Thruster_L1`) 1 (`self.DynMat_RocketFlare1`))
  (`PrimitiveComponent.SetMaterial` (`self.SM_Frigate_MB3_Thruster_R1`) 1 (`self.DynMat_RocketFlare1`))
  (`PrimitiveComponent.SetMaterial` (`self.SM_Frigate_MB3_Thruster_R2`) 1 (`self.DynMat_RocketFlare1`))
  (`PrimitiveComponent.SetMaterial` _sm_frigate_mb3_thruster_l2 2 (`self.DynMat_RocketFlare2`))
  (`PrimitiveComponent.SetMaterial` (`self.SM_Frigate_MB3_Thruster_L1`) 2 (`self.DynMat_RocketFlare2`))
  (`PrimitiveComponent.SetMaterial` (`self.SM_Frigate_MB3_Thruster_R1`) 2 (`self.DynMat_RocketFlare2`))
  (`PrimitiveComponent.SetMaterial` (`self.SM_Frigate_MB3_Thruster_R2`) 2 (`self.DynMat_RocketFlare2`))
  (`PrimitiveComponent.SetMaterial` _sm_frigate_mb3_thruster_l2 3 (`self.DynMat_RocketFlare3`))
  (`PrimitiveComponent.SetMaterial` (`self.SM_Frigate_MB3_Thruster_L1`) 3 (`self.DynMat_RocketFlare3`))
  (`PrimitiveComponent.SetMaterial` (`self.SM_Frigate_MB3_Thruster_R1`) 3 (`self.DynMat_RocketFlare3`))
  (`PrimitiveComponent.SetMaterial` (`self.SM_Frigate_MB3_Thruster_R2`) 3 (`self.DynMat_RocketFlare3`))
  (switch `int` (`self.Color`)
    (:`0`
      (`PrimitiveComponent.SetMaterial` _sm_dreadnought_k5_2 0 "/Game/ExtraAsset/SpaceShips_Vol3/Materials/Dreadnought_K5/MI_Dreadnought_K5_Black.MI_Dreadnought_K5_Black")
      (set `self.Thruster_Color` (struct :`R` 1.0 :`B` 0.027019 :`A` 1.0)))
    (:`1`
      (`PrimitiveComponent.SetMaterial` _sm_dreadnought_k5_2 0 "/Game/ExtraAsset/SpaceShips_Vol3/Materials/Dreadnought_K5/MI_Dreadnought_K5_White.MI_Dreadnought_K5_White"))
    (:`2`
      (`PrimitiveComponent.SetMaterial` _sm_dreadnought_k5_2 0 "/Game/ExtraAsset/SpaceShips_Vol3/Materials/Dreadnought_K5/MI_Dreadnought_K5_Yellow.MI_Dreadnought_K5_Yellow")
      (set `self.Thruster_Color` (struct :`R` 1.0 :`G` 0.978421 :`B` 0.72 :`A` 1.0)))
    (:`3`
      (`PrimitiveComponent.SetMaterial` _sm_dreadnought_k5_2 0 "/Game/ExtraAsset/SpaceShips_Vol3/Materials/Dreadnought_K5/MI_Dreadnought_K5_Green.MI_Dreadnought_K5_Green")
      (set `self.Thruster_Color` (struct :`G` 1.0 :`B` 0.89897 :`A` 1.0)))
    (:`4`
      (`PrimitiveComponent.SetMaterial` _sm_dreadnought_k5_2 0 "/Game/ExtraAsset/SpaceShips_Vol3/Materials/Dreadnought_K5/MI_Dreadnought_K5_Red.MI_Dreadnought_K5_Red")
      (set `self.Thruster_Color` (struct :`R` 0.605 :`G` 0.594213 :`B` 0.0847 :`A` 1.0)))
    (:`5`
      (`PrimitiveComponent.SetMaterial` _sm_dreadnought_k5_2 0 "/Game/ExtraAsset/SpaceShips_Vol3/Materials/Dreadnought_K5/MI_Dreadnought_K5_Blue.MI_Dreadnought_K5_Blue")))
  (bind _returnvalue_5 (`PrimitiveComponent.CreateDynamicMaterialInstance` _sm_dreadnought_k5 0 (`PrimitiveComponent.GetMaterial` _sm_dreadnought_k5 0) "None"))
  (bind _output_get (set `self.ShipMaterial` _returnvalue_5))
  (`PrimitiveComponent.SetMaterial` _sm_dreadnought_k5 0 _output_get)
  (`MaterialInstanceDynamic.SetVectorParameterValue` (`self.DynMat_RocketFlare0`) "Color" (`self.Thruster_Color`))
  (`MaterialInstanceDynamic.SetVectorParameterValue` (`self.DynMat_RocketFlare1`) "Color" (`self.Thruster_Color`))
  (`MaterialInstanceDynamic.SetVectorParameterValue` (`self.DynMat_RocketFlare2`) "Color" (`self.Thruster_Color`))
  (`MaterialInstanceDynamic.SetVectorParameterValue` (`self.DynMat_RocketFlare3`) "Color" (`self.Thruster_Color`))
  (`MaterialInstanceDynamic.SetVectorParameterValue` (`self.ShipMaterial`) "ThrusterColor" (`self.Thruster_Color`)))