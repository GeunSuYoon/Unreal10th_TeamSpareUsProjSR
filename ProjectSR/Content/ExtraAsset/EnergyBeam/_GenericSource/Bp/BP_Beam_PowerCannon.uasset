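; Power cannon beam actor whose Niagara beam shortens at the first object it hits, unless set to go through.
; Each tick a sphere trace, grown by a timeline and ignoring the attach parent's owner, sets beam length.
; An optional impact effect follows the hit point, respawning on a new target and deactivating when contact ends.
; Construction applies the look settings, and a shutdown event stops tracing, then destroys the actor only if an impact effect exists.
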(event `InitializeBlockVFX`
  (bind _newvfx (`self.NewVFX`))
  ;[1 1 1] InitializedBlockVFX
  (`/Engine/EditorBlueprintResources/StandardMacros.IsValid` _newvfx
    (:`Is Valid`
      (`NiagaraComponent.SetVariableFloat` _newvfx "DelayTime" (`KismetMathLibrary.SelectFloat` (* (`self.FirstBlockDelay`) (/ (`self.BlockDistance`) (`self.Distance`))) 0.0 (`self.CurrentHit`)))
      (`NiagaraComponent.SetVariableFloat` _newvfx "_ColorHue" (+ (`self._ColorHue`) 0.05))
      (`NiagaraComponent.SetVariableFloat` _newvfx "_Size" (* (`self._Width`) (`self.MyBlockVFX_Size`)))
      (`NiagaraComponent.SetVariableBool` _newvfx "NoAirDistort" (`self.NoAirDistort`))
      (`NiagaraComponent.SetVariableBool` _newvfx "NoDecal" (`self.NoDecalForBlockVFX`)))))

(event `DeActivateThenDestory`
  (bind _newvfx (`self.NewVFX`))
  ;[1 1 1] DeactivateAndDestory
  (set `self.TransitionProgress` 0.0)
  (set `self.CanTrace` false)
  (`ActorComponent.SetActive` (`self.BeamVFX`) false true)
  (`KismetSystemLibrary.Delay` 0.5)
  (`/Engine/EditorBlueprintResources/StandardMacros.IsValid` _newvfx
    (:`Is Valid`
      (`ActorComponent.SetActive` _newvfx false true)
      (`KismetSystemLibrary.Delay` (`self.DelayDestroy`))
      (`self.K2_DestroyActor`))))

(event `ActivateVFX`
  ;[1 1 1] ActivateEvent
  (set `self.CanTrace` true)
  (`ActorComponent.SetActive` (`self.BeamVFX`) true true)
  (bind (_direction _transitionprogress) (`Timeline|Timeline` :!via `PlayFromStart`)
    (:`Update`
      (set `self.TransitionProgress` _transitionprogress))))

(event `self.ReceiveBeginPlay`
  ;[1 1 1] Initial
  (bind _output_get (set `self.BlockDistance` (`self.Distance`)))
  (`NiagaraComponent.SetVariableFloat` (`self.BeamVFX`) "_Length" (* (/ _output_get 1325.0) (`self.LengthAdjustFactor`)))
  (`self.ActivateVFX`)
  (`TimelineComponent.SetPlayRate` (`self.Timeline`) (* 1.0 (`self.CollisionGrowSpeedScale`))))

(event `self.ReceiveTick`
  (params (DeltaSeconds :type "Float (single-precision)"))
  (bind _returnvalue (`self.GetActorForwardVector`))
  (bind _returnvalue_2 (`self.K2_GetActorLocation`))
  (bind _beamvfx (`self.BeamVFX`))
  (bind _newvfx (`self.NewVFX`))
  (bind _newvfx_2 (`self.NewVFX`))
  (bind _distance (`self.Distance`))
  (bind _returnvalue_3 (`SceneComponent.GetAttachParent` (`self.DefaultSceneRoot`)))
  (bind _returnvalue_4 (* (/ (`self.BlockDistance`) 1325.0) (`self.LengthAdjustFactor`)))
  (`|ExecutionSequence`
    (:`then_0`
      ;[1 1 1] Get Hit then Block
      (if (`self.CanTrace`)
        (`/Engine/EditorBlueprintResources/StandardMacros.IsValid` _returnvalue_3
          (:`Is Valid`
            (set `self.Parent` (`ActorComponent.GetOwner` _returnvalue_3)))
          (:`Is Not Valid`
            _))
        (bind (_outhit _returnvalue_5) (`KismetSystemLibrary.SphereTraceSingleForObjects` (+ _returnvalue_2 (* (`self.HeadCut`) _returnvalue)) (+ _returnvalue_2 (* (* (`self.Distance`) (`self.TransitionProgress`)) _returnvalue)) (* (`self._Width`) (`self.CollisionThicknessOffset`)) (`self.SelfTargetTypes`) false (`|MakeArray` (`self.Parent`))))
        (if _returnvalue_5
          (if (`self.GoThrough`)
            (set `self.BlockDistance` _distance)
            (else
              (bind (_bblockinghit _binitialoverlap _time _distance_2 _location _impactpoint _normal _impactnormal _physmat _hitactor) (`GameplayStatics.BreakHitResult` _outhit))
              (set `self.BlockDistance` _distance_2)))
          (`NiagaraComponent.SetVariableFloat` _beamvfx "_Length" _returnvalue_4)
          (if (`self.BlockVfxON`)
            (bind _output_get (set `self.NewHitActor` (!= (`self.MyHitActor`) _hitactor)))
            (set `self.MyHitActor` _hitactor)
            (if (or _output_get (== (`self.CurrentHit`) false))
              (bind _output_get_2 (set `self.OldVFX` (`self.NewVFX`)))
              (bind _returnvalue_6 (`NiagaraFunctionLibrary.SpawnSystemAtLocation` (`self.MyBlockVFX`)))
              (set `self.NewVFX` _returnvalue_6)
              (`self.InitializeBlockVFX`)
              (`/Engine/EditorBlueprintResources/StandardMacros.IsValid` _output_get_2
                (:`Is Valid`
                  (`ActorComponent.Deactivate` _output_get_2))
                (:`Is Not Valid`
                  _)))
            (`/Engine/EditorBlueprintResources/StandardMacros.IsValid` _newvfx
              (:`Is Valid`
                (`SceneComponent.K2_SetWorldLocation` _newvfx (+ _location (* (`self.BlockLocationOffset`) _impactnormal)) false true)
                (set `self.CurrentHit` true))))
          (else
            (set `self.BlockDistance` _distance)
            (`NiagaraComponent.SetVariableFloat` _beamvfx "_Length" _returnvalue_4)
            (set `self.CurrentHit` false)
            (`/Engine/EditorBlueprintResources/StandardMacros.IsValid` _newvfx_2
              (:`Is Valid`
                (`ActorComponent.Deactivate` _newvfx_2)))))))))

(fn `UserConstructionScript`
  (bind _beamvfx (`self.BeamVFX`))
  (`NiagaraComponent.SetVariableBool` _beamvfx "Optimized" (`self.Optimized`))
  (`NiagaraComponent.SetVariableBool` _beamvfx "NoAirDistort" (`self.NoAirDistort`))
  (`NiagaraComponent.SetVariableBool` _beamvfx "AudioON" (`self.AudioON`))
  (`NiagaraComponent.SetVariableFloat` _beamvfx "_Length" (* (/ (`self.Distance`) 1325.0) (`self.LengthAdjustFactor`)))
  (`NiagaraComponent.SetVariableFloat` _beamvfx "_Size" 1.0)
  (`NiagaraComponent.SetVariableFloat` _beamvfx "_ColorHue" (`self._ColorHue`))
  (`NiagaraComponent.SetVariableFloat` _beamvfx "_Width" (`self._Width`)))