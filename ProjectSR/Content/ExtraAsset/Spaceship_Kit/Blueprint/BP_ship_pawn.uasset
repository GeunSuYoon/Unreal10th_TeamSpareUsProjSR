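; BP_ship_pawn is a player-controlled spaceship pawn with physics-driven flight.
; BeginPlay adds the IMC_Ship Enhanced Input mapping context for player 0.
; Tick overwrites ShipRoot's linear velocity along its forward vector, scaled by Power, which nothing here changes.
; Roll, pitch and yaw inputs apply torque about the ship's local axes as mass-independent acceleration, so steering redirects the constant forward motion.
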(event `self.ReceiveBeginPlay`
  (`EnhancedInputSubsystemInterface.AddMappingContext` (pcsubsystem `EnhancedInputLocalPlayerSubsystem` (`GameplayStatics.GetPlayerController` 0)) "/Game/ExtraAsset/Spaceship_Kit/Input/IMC_Ship.IMC_Ship" 0 (struct)))

(event `self.ReceiveTick`
  (params (DeltaSeconds :type "Float (single-precision)"))
  (`PrimitiveComponent.SetPhysicsLinearVelocity` (`self.Ship_root`) (* (`SceneComponent.GetForwardVector` (`self.Ship_root`)) (`self.Power`) 5.0) false "None"))

(event `EnhancedInput|/Game/ExtraAsset/Spaceship_Kit/Input/IA_RollPitch`
  (params (ActionValue :type "Vector2D Structure") (ElapsedSeconds :type "Float (double-precision)") (TriggeredSeconds :type "Float (double-precision)") (InputAction :type "InputAction Object Reference" :default "/Game/ExtraAsset/Spaceship_Kit/Input/IA_RollPitch.IA_RollPitch"))
  (:`Triggered`
    ;[1 1 1] Roll
    (`PrimitiveComponent.AddTorqueInDegrees` (`self.Ship_root`) (* (`SceneComponent.GetForwardVector` (`self.Ship_root`)) 50.0 (`KismetMathLibrary.BreakVector2D` (`|GetInputActionValue`)) -1.0) "None" true)
    ;[1 1 1] Pitch
    (`PrimitiveComponent.AddTorqueInDegrees` (`self.Ship_root`) (* (`SceneComponent.GetRightVector` (`self.Ship_root`)) 50.0 (`.Y` (`KismetMathLibrary.BreakVector2D` (`|GetInputActionValue`)))) "None" true)))

(event `EnhancedInput|/Game/ExtraAsset/Spaceship_Kit/Input/IA_Yaw`
  (params (ActionValue :type "Float (double-precision)") (ElapsedSeconds :type "Float (double-precision)") (TriggeredSeconds :type "Float (double-precision)") (InputAction :type "InputAction Object Reference" :default "/Game/ExtraAsset/Spaceship_Kit/Input/IA_Yaw.IA_Yaw"))
  (:`Triggered`
    (`PrimitiveComponent.AddTorqueInDegrees` (`self.Ship_root`) (* ActionValue (`SceneComponent.GetUpVector` (`self.Ship_root`)) 80.0) "None" true)))

(fn `UserConstructionScript`)