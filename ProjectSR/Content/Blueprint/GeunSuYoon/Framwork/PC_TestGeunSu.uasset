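; PC_TestGeunSu is a test player controller that turns Enhanced Input actions into pawn movement and camera look.
; On BeginPlay it adds the character action mapping context.
; Move input becomes a normalized direction relative to control-rotation yaw, with X as forward and Y as right, and drives AddMovementInput.
; Mouse look feeds yaw and inverted pitch input, while the interact action is an empty stub.
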(event `self.ReceiveBeginPlay`
  (`EnhancedInputSubsystemInterface.AddMappingContext` (subsystem `EnhancedInputLocalPlayerSubsystem`) "/Game/Blueprint/GeunSuYoon/Framwork/IMC_CharacterActionMapping.IMC_CharacterActionMapping" 0 (struct)))

(event `EnhancedInput|/Game/Input/Actions/IA_Move`
  (params (ActionValue :type "Vector2D Structure") (ElapsedSeconds :type "Float (double-precision)") (TriggeredSeconds :type "Float (double-precision)") (InputAction :type "InputAction Object Reference" :default "/Game/Input/Actions/IA_Move.IA_Move"))
  (bind _returnvalue (`self.K2_GetPawn`))
  (bind (_returnvalue_x _returnvalue_y _returnvalue_z) (`KismetMathLibrary.BreakVector` (`KismetMathLibrary.Conv_Vector2DToVector` ActionValue)))
  (bind _returnvalue_2 (`KismetMathLibrary.MakeRotator` 0.0 0.0 (.yaw (`Pawn.GetControlRotation` _returnvalue))))
  (:`Triggered`
    (bind _output_get (set `self.MoveDir` (`KismetMathLibrary.Normal` (+ (* _returnvalue_x (`KismetMathLibrary.GetForwardVector` _returnvalue_2)) (* _returnvalue_y (`KismetMathLibrary.GetRightVector` _returnvalue_2))))))
    (`Pawn.AddMovementInput` _returnvalue _output_get 300.0 false)))

(event `EnhancedInput|/Game/Input/Actions/IA_MouseLook`
  (params (ActionValue :type "Vector2D Structure") (ElapsedSeconds :type "Float (double-precision)") (TriggeredSeconds :type "Float (double-precision)") (InputAction :type "InputAction Object Reference" :default "/Game/Input/Actions/IA_MouseLook.IA_MouseLook"))
  (bind (_x _y) (`KismetMathLibrary.BreakVector2D` ActionValue))
  (:`Triggered`
    (`self.AddYawInput` _x)
    (`self.AddPitchInput` (* _y -1.0))))

(event `EnhancedInput|/Game/Blueprint/GeunSuYoon/Framwork/IA_Interact`
  (params (ActionValue :type Boolean) (ElapsedSeconds :type "Float (double-precision)") (TriggeredSeconds :type "Float (double-precision)") (InputAction :type "InputAction Object Reference" :default "/Game/Blueprint/GeunSuYoon/Framwork/IA_Interact.IA_Interact")))

(fn `UserConstructionScript`)