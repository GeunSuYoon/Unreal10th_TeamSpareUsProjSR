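; BP_ItemActor is an item actor whose Widget component always faces the player camera.
; Every Tick it rotates the widget with a look-at rotation toward the first player's camera location.
; It then moves the widget to a fixed distance from the actor's origin along the direction to that camera, keeping it on the viewer's side of the item.
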(event `self.ReceiveTick`
  (params (DeltaSeconds :type "Float (single-precision)"))
  (bind _returnvalue (`PlayerCameraManager.GetCameraLocation` (`GameplayStatics.GetPlayerCameraManager` 0)))
  (`SceneComponent.K2_SetWorldRotation` (`self.Widget`) (`KismetMathLibrary.FindLookAtRotation` (`SceneComponent.K2_GetComponentLocation` (`self.Widget`)) _returnvalue) false false)
  (`SceneComponent.K2_SetWorldLocation` (`self.Widget`) (+ (`self.K2_GetActorLocation`) (* (`KismetMathLibrary.Normal` (- _returnvalue (`self.K2_GetActorLocation`))) 100.0)) false false))

(fn `UserConstructionScript`)