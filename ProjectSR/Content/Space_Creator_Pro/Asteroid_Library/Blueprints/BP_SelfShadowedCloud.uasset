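; Placeable volumetric cloud actor that renders a self-shadowed volume texture on a cube mesh.
; The construction script creates a dynamic instance of MI_Volume_SelfShadowed and feeds it the actor's texture, density, shadow and color settings.
; It also passes the negated forward vector of the referenced DirLight as the light direction, which is set only at construction because the event graph is empty.
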(fn `UserConstructionScript`
  (bind _returnvalue (`PrimitiveComponent.CreateDynamicMaterialInstance` (`self.Cube`) 0 "/Game/Space_Creator_Pro/Asteroid_Library/Material_Instances/MI_Volume_SelfShadowed.MI_Volume_SelfShadowed" "None"))
  (set `self.DMI_SelfShadowedCloud` _returnvalue)
  (`MaterialInstanceDynamic.SetTextureParameterValue` (`self.DMI_SelfShadowedCloud`) "T_VOLUME" (`self.Texture`))
  (`MaterialInstanceDynamic.SetScalarParameterValue` (`self.DMI_SelfShadowedCloud`) "Self-Shadow_Distance" (`self.Self-Shadow_Distance`))
  (`MaterialInstanceDynamic.SetScalarParameterValue` (`self.DMI_SelfShadowedCloud`) "Density" (`self.Density`))
  (`MaterialInstanceDynamic.SetScalarParameterValue` (`self.DMI_SelfShadowedCloud`) "ShadowMultiplier" (`self.ShadowMultiplier`))
  (`MaterialInstanceDynamic.SetVectorParameterValue` (`self.DMI_SelfShadowedCloud`) "Color_Lit" (`self.Color_Lit`))
  (`MaterialInstanceDynamic.SetVectorParameterValue` (`self.DMI_SelfShadowedCloud`) "Color_Shadow" (`self.Color_Shadow`))
  (`MaterialInstanceDynamic.SetVectorParameterValue` (`self.DMI_SelfShadowedCloud`) "LightDirection" (`KismetMathLibrary.Conv_VectorToLinearColor` (* (`KismetMathLibrary.Conv_RotatorToVector` (`self.K2_GetActorRotation` (`self.Dir_Light`))) (-1.0 -1.0 -1.0)))))