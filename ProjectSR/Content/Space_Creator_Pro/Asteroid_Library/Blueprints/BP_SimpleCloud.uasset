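; BP_SimpleCloud is a placeable volumetric cloud from the Space Creator Pro asteroid library, drawn with a material on its Cube component.
; The Construction Script creates a dynamic instance of MI_Volume_CloudSimple_1 on the Cube and passes the Blueprint's threshold (spelled "Trenshold"), density and color variables into it.
; The event graph holds only disabled placeholder events, so the Blueprint adds no runtime logic.
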(fn `UserConstructionScript`
  (bind _returnvalue (`PrimitiveComponent.CreateDynamicMaterialInstance` (`self.Cube`) 0 "/Game/Space_Creator_Pro/Asteroid_Library/Material_Instances/MI_Volume_CloudSimple_1.MI_Volume_CloudSimple_1" "None"))
  (set `self.DMI_SelfShadowedCloud` _returnvalue)
  (`MaterialInstanceDynamic.SetScalarParameterValue` (`self.DMI_SelfShadowedCloud`) "Trenshold" (`self.Trenshold`))
  (`MaterialInstanceDynamic.SetScalarParameterValue` (`self.DMI_SelfShadowedCloud`) "Density" (`self.Density`))
  (`MaterialInstanceDynamic.SetVectorParameterValue` (`self.DMI_SelfShadowedCloud`) "Color" (`self.Color`)))