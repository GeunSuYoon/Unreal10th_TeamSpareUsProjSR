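; Construction-script actor that builds a globular asteroid field from four configurable meshes, using either their default materials or overrides.
; Each cluster iteration picks a separate random center per mesh and scatters a quarter of the asteroid count there as instanced static mesh instances.
; Random directions with power-curved distances shape both cluster and asteroid spread, with random rotation and uniform scale per instance.
; Randomness is unseeded, so the layout changes on each reconstruction.
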(fn `BPF_AsteroidCluster`
  (params (`Instanced Static Mesh` :type "InstancedStaticMeshComponent Object Reference") (`Cluster Location` :type "Vector Structure") (`Number Of Asteroids` :type Integer) (`Asteroids Distance` :type "Float (double-precision)") (`Asteroids Distance Distribution` :type "Float (double-precision)") (`Asteroid Scale` :type "Float (double-precision)") (`Asteroid Scale Variation` :type "Float (double-precision)"))
  (for _ (range `Number Of Asteroids`)
    (`InstancedStaticMeshComponent.AddInstance` `Instanced Static Mesh` (`KismetMathLibrary.MakeTransform` (+ `Cluster Location` (* (`KismetMathLibrary.RandomUnitVector`) (* `Asteroids Distance` (`KismetMathLibrary.MultiplyMultiply_FloatFloat` (`KismetMathLibrary.RandomFloatInRange` 0.0 1.0) `Asteroids Distance Distribution`)))) (`KismetMathLibrary.RandomRotator` true) (`KismetMathLibrary.Conv_DoubleToVector` (* `Asteroid Scale` (`KismetMathLibrary.RandomFloatInRange` (/ 1.0 `Asteroid Scale Variation`) 1.0)))) false))
  (return))

(fn `UserConstructionScript`
  (bind _sm_1 (`self.SM 1`))
  (bind _sm_2 (`self.SM 2`))
  (bind _sm_3 (`self.SM 3`))
  (bind _sm_4 (`self.SM 4`))
  (bind _returnvalue (`StaticMesh.GetMaterial` _sm_4 0))
  (bind _returnvalue_2 (`StaticMesh.GetMaterial` _sm_1 0))
  (bind _returnvalue_3 (`StaticMesh.GetMaterial` _sm_2 0))
  (bind _returnvalue_4 (`StaticMesh.GetMaterial` _sm_3 0))
  (bind _returnvalue_5 (* (`KismetMathLibrary.RandomUnitVector`) (* (`self.Clusters Distance`) (`KismetMathLibrary.MultiplyMultiply_FloatFloat` (`KismetMathLibrary.RandomFloatInRange` 0.0 1.0) (`self.Clusters Distance Distribution`)))))
  (`StaticMeshComponent.SetStaticMesh` (`self.ISM_Asteroid_1`) _sm_1)
  (`StaticMeshComponent.SetStaticMesh` (`self.ISM_Asteroid_2`) _sm_2)
  (`StaticMeshComponent.SetStaticMesh` (`self.ISM_Asteroid_3`) _sm_3)
  (`StaticMeshComponent.SetStaticMesh` (`self.ISM_Asteroid_4`) _sm_4)
  (if (`self.Use Default Material`)
    (set `self.Material_Mesh_1` _returnvalue_2)
    (set `self.Material_Mesh_2` _returnvalue_3)
    (set `self.Material_Mesh_3` _returnvalue_4)
    (set `self.Material_Mesh_4` _returnvalue)
    (`PrimitiveComponent.SetMaterial` (`self.ISM_Asteroid_1`) 0 _returnvalue_2)
    (`PrimitiveComponent.SetMaterial` (`self.ISM_Asteroid_2`) 0 _returnvalue_3)
    (`PrimitiveComponent.SetMaterial` (`self.ISM_Asteroid_3`) 0 _returnvalue_4)
    (`PrimitiveComponent.SetMaterial` (`self.ISM_Asteroid_4`) 0 _returnvalue)
    (else
      (`PrimitiveComponent.SetMaterial` (`self.ISM_Asteroid_1`) 0 (`self.Material_Mesh_1`))
      (`PrimitiveComponent.SetMaterial` (`self.ISM_Asteroid_2`) 0 (`self.Material_Mesh_2`))
      (`PrimitiveComponent.SetMaterial` (`self.ISM_Asteroid_3`) 0 (`self.Material_Mesh_3`))
      (`PrimitiveComponent.SetMaterial` (`self.ISM_Asteroid_4`) 0 (`self.Material_Mesh_4`))))
  (for _ (range (`self.Number of Clusters`))
    (`self.BPF_AsteroidCluster` (`self.ISM_Asteroid_1`) _returnvalue_5 (/ (`self.Number of Asteroids`) 4) (`self.Asteroid Distance`) (`self.Asteroid Distance Distribution`) (`self.Asteroid Scale`) (`self.Asteroid Scale Variation Fraction`))
    (`self.BPF_AsteroidCluster` (`self.ISM_Asteroid_2`) _returnvalue_5 (/ (`self.Number of Asteroids`) 4) (`self.Asteroid Distance`) (`self.Asteroid Distance Distribution`) (`self.Asteroid Scale`) (`self.Asteroid Scale Variation Fraction`))
    (`self.BPF_AsteroidCluster` (`self.ISM_Asteroid_3`) _returnvalue_5 (/ (`self.Number of Asteroids`) 4) (`self.Asteroid Distance`) (`self.Asteroid Distance Distribution`) (`self.Asteroid Scale`) (`self.Asteroid Scale Variation Fraction`))
    (`self.BPF_AsteroidCluster` (`self.ISM_Asteroid_4`) _returnvalue_5 (/ (`self.Number of Asteroids`) 4) (`self.Asteroid Distance`) (`self.Asteroid Distance Distribution`) (`self.Asteroid Scale`) (`self.Asteroid Scale Variation Fraction`))))